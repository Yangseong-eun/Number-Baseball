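; Chat controller that links a player's chat window to the game mode and holds that player's user ID.
; On BeginPlay, when the remote role is not None, it waits briefly, then binds an event to the first Widget_ChatWindow.
; Login passes on and stores the user ID, which prefixes outgoing messages handed to BP_ChatMode.
; Received broadcasts print to screen only with authority.
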(event `self.ReceiveBeginPlay`
  ; 게임이 시작될 때 특정 위젯(채팅창)을 찾고,
  ; 이 위젯을 User Controller와 연결하여 메시지를 서버로 전송하는 이벤트를 바인딩하는 역할
  (if (not (`|EnumEquality` (`self.GetRemoteRole`) "ROLE_None"))
    (`KismetSystemLibrary.Delay` 0.5)
    (bind _foundwidgets (`WidgetBlueprintLibrary.GetAllWidgetsOfClass` "/Game/Widgets/Widget_ChatWindow.Widget_ChatWindow_C"))
    (bind _output_get (set `self.Widget` (`|GetArrayItem` _foundwidgets)))
    (bind _aswidget_chat_window (cast `/Game/Widgets/Widget_ChatWindow` _output_get))
    (add `/Game/Widgets/Widget_ChatWindow.SetMessageToUserController` _aswidget_chat_window (`|CreateDelegate` :!event `OnSendMsgToServer`))))

(event `OnLoginWithID`
  (params (UserId :type String))
  ; 서버에서 실행되는 OnLoginWithID 이벤트가 호출되면, 해당 플레이어의 User ID를 설정하고 로그인 처리
  (`self.OnUserLogin` UserId)
  (set `self.UserId` UserId))

(event `GotBroadcast`
  (params (Msg :type String))
  ; 클라이언트에서 특정 메시지를 받을 때 그 메시지를 출력하기 전에 서버인지 클라이언트인지 확인하는 역할
  (if (`self.HasAuthority`)
    (`KismetSystemLibrary.PrintString` Msg true true (struct :`G` 0.66 :`B` 1.0 :`A` 1.0) 10.0)))

(event `OnSendMsgToServer`
  (params (Msg :type String))
  ; 플레이어가 입력한 메시지를 서버에 보내고, 서버가 이를 처리하여 게임 내 채팅 기능을 동작하게 함.
  (bind _asbp_chat_mode (cast `/Game/GameModes/BP_ChatMode` (`GameplayStatics.GetGameMode`)))
  (`/Game/GameModes/BP_ChatMode.GotMessageFromClient` _asbp_chat_mode (`KismetStringLibrary.Concat_StrStr` (`self.UserId`) ":" Msg)))

(fn `UserConstructionScript`)