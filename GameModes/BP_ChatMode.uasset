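; Chat-driven game mode for a two-player number baseball game, where Host and Guest guess a random secret number.
; BeginPlay generates the secret, and GotMessageFromClient strips the sender prefix, validates each guess and scores it as strikes and balls.
; Per-player tries, a host-turn flag and strike counters drive game-over and reset checks.
; Only the guest branch broadcasts scores to every BP_Controller; host scores are just printed.
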(event `self.ReceiveBeginPlay`
  (bind _returnvalue (`GuessNumberLogic.GenerateRandomNumber`))
  (bind _output_get (set `self.SecretNumber` _returnvalue))
  (`KismetSystemLibrary.PrintString` _output_get))

(event `GotMessageFromClient`
  (params (Msg :type String))
  (bind _returnvalue (`KismetStringLibrary.Contains` Msg "Host:"))
  (bind _returnvalue_2 (`KismetMathLibrary.SelectString` "Host:" "Guest:" _returnvalue))
  (bind _returnvalue_3 (`KismetStringLibrary.RightChop` (`KismetStringLibrary.Replace` Msg _returnvalue_2) 2))
  (bind _returnvalue_4 (`KismetStringLibrary.RightChop` (`KismetStringLibrary.Replace` Msg _returnvalue_2) 1))
  (if (or (> (`self.GuestTries`) 0) (> (`self.HostTries`) 0))
    (if _returnvalue
      (`KismetSystemLibrary.PrintString` _returnvalue_4)
      (bind _output_get (set `self.PlayerGuess` _returnvalue_4))
      (bind _returnvalue_5 (`GuessNumberLogic.IsValidGuess` _output_get))
      (if _returnvalue_5
        (set `self.bIsHostTurn` true)
        (bind (_outstrikes _outballs) (`GuessNumberLogic.EvaluateGuess` (`self.SecretNumber`) (`self.PlayerGuess`)))
        (`KismetSystemLibrary.PrintString` (`KismetStringLibrary.Concat_StrStr` (`KismetStringLibrary.Conv_IntToString` _outstrikes) "S" (`KismetStringLibrary.Conv_IntToString` _outballs) "B"))
        (if (`self.bIsHostTurn`)
          (set `self.HostTries` (- (`self.HostTries`) 1))
          (if (== (`self.HostTries`) 0)
            (`KismetSystemLibrary.PrintString` "게임 종료")
            (else
              (bind (_hosttries _guesttries _outnewsecretnumber _bgamereset) (`GuessNumberLogic.CheckGameResult` (`self.HostStrikes`) (`self.GuestStrikes`)))
              (if _bgamereset
                (if (== (`self.HostStrikes`) 3)
                  (bind (_outnewsecretnumber_2 _outhosttries _outguesttries) (`GuessNumberLogic.ResetGame`))
                  (bind _output_get_2 (set `self.SecretNumber` _outnewsecretnumber_2))
                  (set `self.HostTries` _outhosttries)
                  (set `self.GuestTries` _outguesttries)
                  (`KismetSystemLibrary.PrintString` _output_get_2))))))
        (else
          (`KismetSystemLibrary.PrintString` "잘못된 입력입니다")))
      (elif (not (`KismetStringLibrary.Contains` "" "uest:"))
        (`KismetSystemLibrary.PrintString` _returnvalue_3)
        (bind _output_get_3 (set `self.PlayerGuess` _returnvalue_3))
        (bind _returnvalue_6 (`GuessNumberLogic.IsValidGuess` _output_get_3))
        (if _returnvalue_6
          (bind (_outstrikes_2 _outballs_2) (`GuessNumberLogic.EvaluateGuess` (`self.SecretNumber`) (`self.PlayerGuess`)))
          (if (`self.bIsHostTurn`)
            _
            (elif (not (== _outstrikes_2 3))
              (set `self.GuestStrikes` (+ (`self.GuestStrikes`) 1))
              (if (== (`self.GuestStrikes`) 3)
                (bind _outnewsecretnumber_3 (`GuessNumberLogic.ResetGame`))
                (`KismetSystemLibrary.PrintString` _outnewsecretnumber_3)
                (bind _outactors (`GameplayStatics.GetAllActorsOfClass` "/Script/Engine.PlayerController" :!label _label))
                (for _array_element _outactors
                  (bind _asbp_controller (cast `/Game/Blueprints/BP_Controller` _array_element))
                  (`/Game/Blueprints/BP_Controller.GotBroadcast` _asbp_controller (`KismetStringLibrary.Concat_StrStr` (`KismetStringLibrary.Conv_IntToString` _outstrikes_2) "S" (`KismetStringLibrary.Conv_IntToString` _outballs_2) "B")))
                (else
                  (set `self.GuestTries` (- (`self.GuestTries`) 1))
                  (if (== (`self.GuestTries`) 0)
                    (`KismetSystemLibrary.PrintString` "게임 종료")
                    (else
                      (bind (_hosttries_2 _guesttries_2 _outnewsecretnumber_4 _bgamereset_2) (`GuessNumberLogic.CheckGameResult` (`self.HostStrikes`) (`self.GuestStrikes`)))
                      (if _bgamereset_2
                        _
                        (elif (== (`self.GuestStrikes`) 3)
                          (bind (_outnewsecretnumber_5 _outhosttries_2 _outguesttries_2) (`GuessNumberLogic.ResetGame`))
                          (bind _output_get_4 (set `self.SecretNumber` _outnewsecretnumber_5))
                          (set `self.HostTries` _outhosttries_2)
                          (set `self.GuestTries` _outguesttries_2)
                          (`KismetSystemLibrary.PrintString` _output_get_4)
                          (goto _label)
                          (else
                            (goto _label)))))))))))))
    (else
      (`KismetSystemLibrary.PrintString` "기회 소진"))))

(fn `UserConstructionScript`)